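; Player controller for LaoRTS that moves the controlled pawn by axis input, with unfinished mouse edge scrolling as a fallback.
; MoveForward and MoveRight apply movement along control-rotation yaw, substituting the mouse scales when axis input is zero.
; MouseMovement prints normalized cursor position and sets a graded leftward scale between two edge thresholds.
; Disconnected logic holds four-edge scrolling, so the live graph never updates the forward mouse scale.
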(event EventBeginPlay)

(event EventTick
  (params (DeltaSeconds :type Float%20%28single-precision%29)))

(event Input|AxisEvents|InputAxisMouseMovement
  (params (AxisValue :type Float%20%28single-precision%29))
  (bind (_locationx _locationy) (Game|Player|GetMousePosition))
  (bind _returnvalue (Viewport|GetViewportSize))
  (bind _locationx_2 (Game|Player|GetMousePosition))
  (bind _returnvalue_2 (Viewport|GetViewportSize))
  (bind _innerviewport_edge_threshold (Variables|Default|GetInnerViewport%20Edge%20Threshold))
  (bind _outerviewportedgethreshold (Variables|Default|GetOuterViewportEdgeThreshold))
  (bind _returnvalue_3 (/ _locationx_2 (.x _returnvalue_2)))
  ;[1 1 1] debugger
  (Development|PrintString (Utilities|String|Append (Utilities|String|ToString(Float) (/ _locationx (.x _returnvalue))) "" (Utilities|String|ToString(Float) (/ _locationy (.y _returnvalue)))) true true "(R=0.000000,G=0.660000,B=1.000000,A=1.000000)" 0.0)
  (Variables|Default|SetMouseRightScale (Math|Float|SelectFloat (* (/ (- _innerviewport_edge_threshold _returnvalue_3) (- _innerviewport_edge_threshold _outerviewportedgethreshold)) -1.0) 0.0 (and (>= _returnvalue_3 _outerviewportedgethreshold) (<= _returnvalue_3 _innerviewport_edge_threshold)))))

(event Input|AxisEvents|InputAxisMoveForward
  (params (AxisValue :type Float%20%28single-precision%29))
  (Pawn|Input|AddMovementInput (Pawn|GetControlledPawn) (Math|Vector|GetForwardVector (Math|Rotator|MakeRotator 0.0 0.0 (.yaw (Pawn|GetControlRotation :!class /Script/Engine.Controller)))) (Math|Float|SelectFloat AxisValue (Variables|Default|GetMouseForwardScale) (!= AxisValue 0.0)) false))

(event Input|AxisEvents|InputAxisMoveRight
  (params (AxisValue :type Float%20%28single-precision%29))
  (Pawn|Input|AddMovementInput (Pawn|GetControlledPawn) (Math|Vector|GetRightVector (Math|Rotator|MakeRotator 0.0 0.0 (.yaw (Pawn|GetControlRotation :!class /Script/Engine.Controller)))) (Math|Float|SelectFloat AxisValue (Variables|Default|GetMouseRightScale) (!= AxisValue 0.0)) false))

(fn ConstructionScript)